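; ChessHUD_BP is the chess game's HUD Blueprint, which creates and holds its UI widgets on BeginPlay.
; It adds both players' point widgets, the 2D projection view and the material switching tab to the viewport for player controller 0.
; It also creates the winning screen and replay widget without displaying them, and passes the replay widget to the winning screen as its ReplayScreen.
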(event `self.ReceiveBeginPlay`
  (bind _returnvalue (`GameplayStatics.GetPlayerController` 0))
  ;[1 1 1] Adding Player1PointBP to ViewPort
  (bind _returnvalue_2 (`|CreateWidget` "/Game/Blueprint/Player1Point_BP.Player1Point_BP_C" _returnvalue))
  (bind _output_get (set `self.widgetPoint1` _returnvalue_2))
  (`UserWidget.AddToViewport` _returnvalue_2 0)
  ;[1 1 1] Adding Player2PointBP to ViewPort
  (bind _returnvalue_3 (`|CreateWidget` "/Game/Blueprint/Player2Point_BP.Player2Point_BP_C" _returnvalue))
  (bind _output_get_2 (set `self.widgetPoint2` _returnvalue_3))
  (`UserWidget.AddToViewport` _output_get_2 0)
  (set `ChessPointsWidget.PlayerPointTextBlock` (`ChessPointsWidget.PlayerPointTextBlock` _output_get) _output_get)
  (set `ChessPointsWidget.PlayerPointTextBlock` (`ChessPointsWidget.PlayerPointTextBlock` _output_get_2) _output_get_2)
  ;[1 1 1] Assigning Projection 2D Widget
  (bind _returnvalue_4 (`|GenericCreateObject` "/Game/Blueprint/Projection2D_bP.Projection2D_BP_C" _returnvalue))
  (set `self.projection2DWidget` _returnvalue_4)
  (`UserWidget.AddToViewport` _returnvalue_4 0)
  ;[1 1 1] Assinging Material Switching Tab
  (bind _returnvalue_5 (`|GenericCreateObject` "/Game/Blueprint/MaterialSwitch.MaterialSwitch_C" _returnvalue))
  (set `self.MaterialSwitchingTab` _returnvalue_5)
  (`UserWidget.AddToViewport` _returnvalue_5 0)
  ;[1 1 1] Assigning Winning Screen
  (bind _returnvalue_6 (`|CreateWidget` "/Game/Blueprint/WinningScreen.WinningScreen_C" _returnvalue))
  (set `self.winningScreen` _returnvalue_6)
  ;[1 1 1] Assigning Replay Widget
  (bind _returnvalue_7 (`|CreateWidget` "/Game/Blueprint/ReplayChessUserWidgetBP.ReplayChessUserWidgetBP_C" _returnvalue))
  (set `self.replayUserWidget` _returnvalue_7)
  (set `WinningScreenWidget.ReplayScreen` _returnvalue_7 _returnvalue_6))

(fn `UserConstructionScript`)